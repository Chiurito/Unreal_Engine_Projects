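; BP_Character1 is a player character Blueprint with mouse look, keyboard movement and an optional double jump.
; Axis inputs drive controller pitch and yaw, and add movement along the actor's forward and right vectors.
; When CanDoubleJump is set, a DoN counter makes the first press a normal Jump and the second an additive upward LaunchCharacter by DoubleJumpForce, resetting on landing.
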(event `InputAxis|LookUp`
  (params (AxisValue :type "Float (single-precision)"))
  ;[1 1 1] Mouse Look
  (`self.AddControllerPitchInput` AxisValue))

(event `InputAxis|Move Forward/Backward`
  (params (AxisValue :type "Float (single-precision)"))
  ;[1 1 1] Keyboard Movement
  (`self.AddMovementInput` (`self.GetActorForwardVector`) AxisValue))

(event `InputAxis|Turn`
  (params (AxisValue :type "Float (single-precision)"))
  ;[1 1 1] Mouse Look
  (`self.AddControllerYawInput` AxisValue))

(event `InputAxis|Move Left/Right`
  (params (AxisValue :type "Float (single-precision)"))
  ;[1 1 1] Keyboard Movement
  (`self.AddMovementInput` (`self.GetActorRightVector`) AxisValue))

(event `InputAction|Jump`
  (params (Key :type "Key Structure"))
  ;[1 1 1] Jump/Double Jump
  (:`Pressed`
    (if (`self.CanDoubleJump`)
      (bind _counter (`/Engine/EditorBlueprintResources/StandardMacros.Do N` 2 :!label _label)
        (:`Exit`
          (switch `int` _counter
            (:`1`
              (`self.Jump`))
            (:`2`
              (`self.LaunchCharacter` (`KismetMathLibrary.MakeVector` 0.0 0.0 (`self.DoubleJumpForce`)))))))
      (else
        (`self.Jump`)))))

(event `self.OnLanded`
  (params (Hit :type "HitResult Structure (by ref)"))
  ;[1 1 1] Jump/Double Jump
  (goto _label :!via `Reset`))

(fn `UserConstructionScript`)