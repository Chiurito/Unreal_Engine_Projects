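; Alien enemy character that chases the player and melee attacks in range until killed.
; BeginPlay runs a repeating AI MoveTo toward the player, retrying after success or failure.
; Tick checks range, alive state and montage playback, pausing movement during attacks; DamagePlayer applies hit damage but is not called here.
; Damage lowers clamped health; death disables movement and collision, credits BP_Marine's kill, notifies GM_MarsMarine, then destroys the actor after a delay.
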(event `self.ReceiveBeginPlay`
  ;[1 0.2526 0.1729] MESH NAVIGATION
  (if (`self.Is Alive`)
    ;;[1 1 1] If player is in the nav mesh (on success pin) or outside the nav mesh (on fail) the ai loop the function move to.
    (`|AIMoveTo` self (0.0 0.0 0.0) (`GameplayStatics.GetPlayerCharacter` 0) :!label _label
      (:`OnSuccess`
        _)
      (:`OnFail`
        _))
    (`KismetSystemLibrary.Delay` 0.2)
    (goto _label)))

(event `self.ReceiveTick`
  (params (DeltaSeconds :type "Float (single-precision)"))
  ;[0.3735 0.5512 1] ALIEN ATTACK. Deactivate character movement and play montage if the alien is in his attack range and not attacking (currently not playing the montage already). On montage play completed reactivate alien movement
  (if (`self.Can Attack`)
    (`ActorComponent.Deactivate` (`self.CharacterMovement`))
    (`|PlayMontage` (`self.Mesh`) "/Game/Characters/Enemy_Great_Spider/Animations/AlienAttack1.AlienAttack1"
      (:`OnCompleted`
        (`ActorComponent.Activate` (`self.CharacterMovement`) false)))))

(event `self.ReceiveAnyDamage`
  (params (Damage :type "Float (single-precision)") (DamageType :type "DamageType Object Reference") (InstigatedBy :type "Controller Object Reference") (DamageCauser :type "Actor Object Reference"))
  (if (`self.Is Alive`)
    (bind _current_health (`self.Decrease Health` Damage))
    (if (== _current_health 0.0)
      (`self.Kill AI`)
      (`KismetSystemLibrary.Delay` 3.0)
      (`self.K2_DestroyActor`))))

(fn `Can Attack`
  (returns (ReturnValue :type Boolean))
  (return (and (`self.Is Within Attack Range`) (not (`self.Is Attacking`)) (`self.Is Alive`))))

(fn `Damage Player`
  (if (`self.Is Alive`)
    (`GameplayStatics.ApplyDamage` (`GameplayStatics.GetPlayerCharacter` 0) (`self.Damage Per Hit`))))

(fn `Deactivate AI Movement`
  (bind _charactermovement (`self.CharacterMovement`))
  (`MovementComponent.StopMovementImmediately` _charactermovement)
  (`ActorComponent.Deactivate` _charactermovement))

(fn `Decrease Health`
  (params (`Damage Amount` :type "Float (double-precision)"))
  (returns (`Current Health` :type "Float (double-precision)"))
  (bind _output_get (set `self.Health` (`KismetMathLibrary.FClamp` (- (`self.Health`) `Damage Amount`) 0.0 100.0)))
  (return _output_get))

(fn `Is Alive`
  (returns (ReturnValue :type Boolean))
  (return (not (`self.Dead`))))

(fn `Is Attacking`
  (returns (ReturnValue :type Boolean))
  (return (`AnimInstance.Montage_IsPlaying` (`SkeletalMeshComponent.GetAnimInstance` (`self.Mesh`)) "/Game/Characters/Enemy_Great_Spider/Animations/AlienAttack1.AlienAttack1")))

(fn `Is Within Attack Range`
  (returns (ReturnValue :type Boolean))
  (return (< (`self.GetDistanceTo` (`GameplayStatics.GetPlayerCharacter` 0)) (`self.Attack Range`))))

(fn `Kill AI`
  (set `self.Dead` true)
  (`self.Deactivate AI Movement`)
  (`self.SetActorEnableCollision` false)
  (bind _asbp_marine (cast `/Game/Blueprints/Pawns/BP_Marine` (`GameplayStatics.GetPlayerCharacter` 0)))
  (`/Game/Blueprints/Pawns/BP_Marine.Increse Kills` _asbp_marine)
  (bind _asgm_mars_marine (cast `/Game/Blueprints/GameMode/GM_MarsMarine` (`GameplayStatics.GetGameMode`)))
  (`/Game/Blueprints/GameMode/GM_MarsMarine.Register Alien Death` _asgm_mars_marine self))

(fn `UserConstructionScript`)