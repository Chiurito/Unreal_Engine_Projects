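; BP_Marine is the player character, a marine with world-axis movement, twin-stick style aiming, a rifle and health.
; Tick sets control-rotation yaw from thumbstick direction or smoothed mouse velocity, both deadzoned, switching on the last key's device.
; Firing toggles muzzle flash and looping sound, with one debug-drawn muzzle trace per press whose hit is unused.
; Damage lowers clamped health; zero sets Dead, which blocks movement and aiming; BeginPlay creates the HUD.
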(event `self.ReceiveAnyDamage`
  (params (Damage :type "Float (single-precision)") (DamageType :type "DamageType Object Reference") (InstigatedBy :type "Controller Object Reference") (DamageCauser :type "Actor Object Reference"))
  ;[1 0.8363 0.0916] DAMAGE SYSTEM
  (bind _current_health (`self.Decrease Health` Damage))
  (if (== _current_health 0.0)
    (set `self.Dead` true)
    (`self.Stop Firing Weapon`)))

(event `self.ReceiveBeginPlay`
  ;[1 0.8085 0.09327] Create HUD Canvas for BP_Marine
  (bind _returnvalue (`|CreateWidget` "/Game/UI/W_PlayerHud.W_PlayerHUD_C" null self))
  (`UserWidget.AddToViewport` _returnvalue 0))

(event `self.ReceiveTick`
  (params (DeltaSeconds :type "Float (single-precision)"))
  ;[1 0.8492 0.03035] Update Animations
  (`self.Update Player Aim`))

(event `InputAxis|MoveForward`
  (params (AxisValue :type "Float (single-precision)"))
  ;[1 0.9046 0.1667] Player Movement only if alive
  (if (`self.Is Alive`)
    (`self.AddMovementInput` (1.0 0.0 0.0) AxisValue)))

(event `Key|AnyKey`
  (params (Key :type "Key Structure"))
  ;[0.8796 0.7176 0.1079] Switch from Gamepad and Mouse rotation
  (:`Pressed`
    (set `self.IsGamepadActive` (`KismetInputLibrary.Key_IsGamepadKey` Key))))

(event `InputAxis|MoveRight`
  (params (AxisValue :type "Float (single-precision)"))
  ;[1 0.9046 0.1667] Player Movement only if alive
  (if (`self.Is Alive`)
    (`self.AddMovementInput` (0.0 1.0 0.0) AxisValue)))

(event `InputAction|Fire Weapon`
  (params (Key :type "Key Structure"))
  ;[1 0.7909 0.07902] Player fire weapon
  (:`Pressed`
    (`self.Start Firing Weapon`)
    (`self.Weapon Trace`))
  (:`Released`
    (`self.Stop Firing Weapon`)))

(fn `Decrease Health`
  (params (`Damage amount` :type "Float (double-precision)"))
  (returns (`Current Health` :type "Float (double-precision)"))
  (bind _output_get (set `self.Player Health` (`KismetMathLibrary.FClamp` (- (`self.Player Health`) `Damage amount`) 0.0 100.0)))
  (return _output_get))

(fn `Get Mouse Aim Direction`
  (returns (ReturnValue :type "Rotator Structure"))
  (bind (_mousevelocity_x _mousevelocity_y) (`KismetMathLibrary.BreakVector2D` (`self.Get Mouse Velocity`)))
  (return (`KismetMathLibrary.RInterpTo` (`Controller.GetControlRotation` (`GameplayStatics.GetPlayerController` 0)) (`KismetMathLibrary.MakeRotator` 0.0 0.0 (`KismetMathLibrary.DegAtan2` _mousevelocity_x _mousevelocity_y)) (`GameplayStatics.GetWorldDeltaSeconds`) (`self.Mouse Smoothing Strenght`))))

(fn `Get Mouse Velocity`
  (returns (MouseVelocity :type "Vector2D Structure"))
  (bind (_deltax _deltay) (`PlayerController.GetInputMouseDelta` (`GameplayStatics.GetPlayerController` 0)))
  (return (/ (`KismetMathLibrary.MakeVector2D` _deltax _deltay) (`GameplayStatics.GetWorldDeltaSeconds`))))

(fn `Get Thumbstick Aim Direction`
  (returns (ReturnValue :type "Rotator Structure"))
  (return (`KismetMathLibrary.MakeRotator` 0.0 0.0 (`KismetMathLibrary.DegAtan2` (`self.GetInputAxisValue`) (`self.GetInputAxisValue`)))))

(fn `Get Weapon End Trace Location`
  (returns (ReturnValue :type "Vector Structure"))
  (return (+ (`self.Get Weapon Trace Start Location`) (* (`KismetMathLibrary.GetForwardVector` (`self.GetControlRotation`)) (`self.Weapon Range`)))))

(fn `Get Weapon Trace Start Location`
  (returns (ReturnValue :type "Vector Structure"))
  (return (`SceneComponent.GetSocketLocation` (`self.RifleMesh`) "MuzzleFlash")))

(fn `Is Alive`
  (returns (ReturnValue :type Boolean))
  (return (not (`self.Dead`))))

(fn `Is Mouse Above Deadzone`
  (returns (ReturnValue :type Boolean))
  (return (> (`KismetMathLibrary.VSize2D` (`self.Get Mouse Velocity`)) (`self.MouseDeadZone`))))

(fn `Is Thumbstick Above Deadzone`
  (returns (ReturnValue :type Boolean))
  (return (> (`KismetMathLibrary.VSize2D` (`KismetMathLibrary.MakeVector2D` (`self.GetInputAxisValue`) (`self.GetInputAxisValue`))) (`self.ThumbstickDeadZone`))))

(fn `Start Firing Weapon`
  (if (`self.Is Alive`)
    (`ActorComponent.Activate` (`self.Muzzle Flash Particle`) false)
    (bind _returnvalue (`GameplayStatics.SpawnSound2D` "/Game/Sounds/Weapon_AssaultRifle/Stereo/RifleFireLoop_Cue.RifleFireLoop_Cue" 1.0 1.0 0.0 null))
    ;[1 1 1] This variable help to stop sound in proper function
    (set `self.Weapon Fire Sound` _returnvalue)))

(fn `Stop Firing Weapon`
  (`ActorComponent.Deactivate` (`self.Muzzle Flash Particle`))
  (`AudioComponent.Stop` (`self.Weapon Fire Sound`))
  (if (`self.Is Alive`)
    (`GameplayStatics.SpawnSound2D` "/Game/Sounds/Weapon_AssaultRifle/Stereo/RifleFireEnd_Cue.RifleFireEnd_Cue" 1.0 1.0 0.0 null)))

(fn `Update Mouse Aim`
  (if (`self.Is Mouse Above Deadzone`)
    (`Controller.SetControlRotation` (`GameplayStatics.GetPlayerController` 0) (`self.Get Mouse Aim Direction`))))

(fn `Update Player Aim`
  (if (`self.Is Alive`)
    (if (`self.IsGamepadActive`)
      (`self.Update Thumbstick Aim`)
      (else
        (`self.Update Mouse Aim`)))))

(fn `Update Thumbstick Aim`
  (if (`self.Is Thumbstick Above Deadzone`)
    (`Controller.SetControlRotation` (`GameplayStatics.GetPlayerController` 0) (`self.Get Thumbstick Aim Direction`))))

(fn `UserConstructionScript`)

(fn `Weapon Trace`
  (`KismetSystemLibrary.LineTraceSingle` :`Start` (`self.Get Weapon Trace Start Location`) :`End` (`self.Get Weapon End Trace Location`) :`TraceChannel` "TraceTypeQuery1" :`DrawDebugType` "ForDuration"))